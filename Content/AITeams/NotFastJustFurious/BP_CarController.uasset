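; AI controller for a NotFastJustFurious car that senses the track and exposes driving controls.
; From BeginPlay, a 0.01-second Delay loop fires debug-drawn line traces around and below the car, horizontal ones at a fixed world height.
; Track hit distances go into an array paired by index with a direction enum array.
; Accelerate, Break and Steer forward values to the AISportsCar pawn; no decision logic here calls them.
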(event `self.ReceivePossess`
  (params (PossessedPawn :type "Pawn Object Reference"))
  (`parent.ReceivePossess` PossessedPawn))

(event `self.ReceiveBeginPlay`
  (bind _controlledcar (`self.ControlledCar`))
  (bind _controlledcar_2 (`self.ControlledCar`))
  (bind _controlledcar_3 (`self.ControlledCar`))
  (bind _controlledcar_4 (`self.ControlledCar`))
  (bind _controlledcar_5 (`self.ControlledCar`))
  (bind _controlledcar_6 (`self.ControlledCar`))
  (bind _controlledcar_7 (`self.ControlledCar`))
  (bind _controlledcar_8 (`self.ControlledCar`))
  (bind _controlledcar_9 (`self.ControlledCar`))
  (bind _controlledcar_10 (`self.ControlledCar`))
  (bind _controlledcar_11 (`self.ControlledCar`))
  (bind _controlledcar_12 (`self.ControlledCar`))
  (bind _controlledcar_13 (`self.ControlledCar`))
  (bind _array (`|MakeArray` (`self.ControlledCar`) :!type "Actor Object Reference"))
  (bind (_returnvalue_x _returnvalue_y) (`KismetMathLibrary.BreakVector` (* (`self.GetActorForwardVector` _controlledcar) 10000)))
  (bind (_returnvalue_x_2 _returnvalue_y_2) (`KismetMathLibrary.BreakVector` (* (`self.GetActorForwardVector` _controlledcar_3) -10000)))
  (bind _returnvalue (`KismetMathLibrary.MakeVector` (.x (`self.K2_GetActorLocation` _controlledcar_12)) (.y (`self.K2_GetActorLocation` _controlledcar_12)) 14.0))
  (bind _returnvalue_2 (`KismetMathLibrary.MakeVector` (.x (`self.K2_GetActorLocation` _controlledcar_4)) (.y (`self.K2_GetActorLocation` _controlledcar_4)) 14.0))
  (bind _returnvalue_3 (`KismetMathLibrary.MakeVector` (.x (`self.K2_GetActorLocation` _controlledcar_5)) (.y (`self.K2_GetActorLocation` _controlledcar_5)) 14.0))
  (bind _returnvalue_4 (`KismetMathLibrary.MakeVector` (.x (`self.K2_GetActorLocation` _controlledcar)) (.y (`self.K2_GetActorLocation` _controlledcar)) 14.0))
  (bind _returnvalue_5 (`KismetMathLibrary.MakeVector` (.x (`self.K2_GetActorLocation` _controlledcar_2)) (.y (`self.K2_GetActorLocation` _controlledcar_2)) 14.0))
  (bind _returnvalue_6 (`KismetMathLibrary.MakeVector` (.x (`self.K2_GetActorLocation` _controlledcar_9)) (.y (`self.K2_GetActorLocation` _controlledcar_9)) 14.0))
  (bind _returnvalue_7 (`KismetMathLibrary.MakeVector` (.x (`self.K2_GetActorLocation` _controlledcar_6)) (.y (`self.K2_GetActorLocation` _controlledcar_6)) 14.0))
  (bind _returnvalue_8 (`KismetMathLibrary.MakeVector` (.x (`self.K2_GetActorLocation` _controlledcar_10)) (.y (`self.K2_GetActorLocation` _controlledcar_10)) 14.0))
  (bind _returnvalue_9 (`KismetMathLibrary.MakeVector` (.x (`self.K2_GetActorLocation` _controlledcar_11)) (.y (`self.K2_GetActorLocation` _controlledcar_11)) 14.0))
  (bind _returnvalue_10 (`KismetMathLibrary.MakeVector` (.x (`self.K2_GetActorLocation` _controlledcar_13)) (.y (`self.K2_GetActorLocation` _controlledcar_13)) 14.0))
  (bind _returnvalue_11 (`KismetMathLibrary.MakeVector` (.x (`self.K2_GetActorLocation` _controlledcar_3)) (.y (`self.K2_GetActorLocation` _controlledcar_3)) 14.0))
  (bind _returnvalue_12 (`KismetMathLibrary.MakeVector` (.x (`self.K2_GetActorLocation` _controlledcar_7)) (.y (`self.K2_GetActorLocation` _controlledcar_7)) 14.0))
  (bind _returnvalue_13 (`KismetMathLibrary.MakeVector` (.x (`self.K2_GetActorLocation` _controlledcar_8)) (.y (`self.K2_GetActorLocation` _controlledcar_8)) 14.0))
  (bind _enumvalue (foreach `ELinecastDirections` false)
    (:`LoopBody`
      (`KismetArrayLibrary.Array_AddUnique` (`self.Directions`) _enumvalue)
      (`KismetArrayLibrary.Array_Add` (`self.Distances`)))
    (:`then`
      (`KismetSystemLibrary.Delay` 0.01 :!label _label)
      (`|ExecutionSequence`
        (:`then_0`
          ;[0 0 0] Front
          (bind (_outhits _returnvalue_14) (`KismetSystemLibrary.LineTraceMultiByProfile` _returnvalue_4 (+ _returnvalue_4 (`KismetMathLibrary.MakeVector` _returnvalue_x _returnvalue_y)) "BlockAll" false _array "ForOneFrame" true (struct :`R` 1.0 :`A` 1.0) (struct :`G` 1.0 :`A` 1.0) 0.05))
          (if _returnvalue_14
            (for _array_element _outhits
              (bind (_bblockinghit _binitialoverlap _time _distance _location _impactpoint _normal _impactnormal _physmat _hitactor) (`GameplayStatics.BreakHitResult` _array_element))
              (if (== (`GameplayStatics.GetObjectClass` _hitactor) "/Game/VehicleTemplate/Blueprints/Track.Track_C")
                (`self.Set Distance In Key` "front" _distance)))))
        (:`then_1`
          ;[0 0 0] Top Right
          (bind (_outhits_2 _returnvalue_15) (`KismetSystemLibrary.LineTraceMultiByProfile` _returnvalue_5 (+ _returnvalue_5 (`KismetMathLibrary.MakeVector` (.x (+ (* (`self.GetActorForwardVector` _controlledcar_2) 4000.0) (* (`self.GetActorRightVector` _controlledcar_2) 4000.0))) (.y (+ (* (`self.GetActorForwardVector` _controlledcar_2) 4000.0) (* (`self.GetActorRightVector` _controlledcar_2) 4000.0))))) "BlockAll" false _array "ForOneFrame" true (struct :`R` 1.0 :`A` 1.0) (struct :`G` 1.0 :`A` 1.0) 0.05))
          (if _returnvalue_15
            (for _array_element_2 _outhits_2
              (bind (_bblockinghit_2 _binitialoverlap_2 _time_2 _distance_2 _location_2 _impactpoint_2 _normal_2 _impactnormal_2 _physmat_2 _hitactor_2) (`GameplayStatics.BreakHitResult` _array_element_2))
              (if (== (`GameplayStatics.GetObjectClass` _hitactor_2) "/Game/VehicleTemplate/Blueprints/Track.Track_C")
                (`self.Set Distance In Key` "topRight" _distance_2)))))
        (:`then_2`
          ;[0 0 0] Top Left
          (bind (_outhits_3 _returnvalue_16) (`KismetSystemLibrary.LineTraceMultiByProfile` _returnvalue_7 (+ _returnvalue_7 (`KismetMathLibrary.MakeVector` (.x (+ (* (`self.GetActorForwardVector` _controlledcar_6) 4000.0) (* (`self.GetActorRightVector` _controlledcar_6) -4000.0))) (.y (+ (* (`self.GetActorForwardVector` _controlledcar_6) 4000.0) (* (`self.GetActorRightVector` _controlledcar_6) -4000.0))))) "BlockAll" false _array "ForOneFrame" true (struct :`R` 1.0 :`A` 1.0) (struct :`G` 1.0 :`A` 1.0) 0.05))
          (if _returnvalue_16
            (for _array_element_3 _outhits_3
              (bind (_bblockinghit_3 _binitialoverlap_3 _time_3 _distance_3 _location_3 _impactpoint_3 _normal_3 _impactnormal_3 _physmat_3 _hitactor_3) (`GameplayStatics.BreakHitResult` _array_element_3))
              (if (== "/Game/VehicleTemplate/Blueprints/Track.Track_C" (`GameplayStatics.GetObjectClass` _hitactor_3))
                (`self.Set Distance In Key` "topLeft" _distance_3)))))
        (:`then_3`
          ;[0 0 0] Top Right 30
          (bind (_outhits_4 _returnvalue_17) (`KismetSystemLibrary.LineTraceMultiByProfile` _returnvalue_12 (+ _returnvalue_12 (`KismetMathLibrary.MakeVector` (.x (+ (* (`self.GetActorForwardVector` _controlledcar_7) 6000.0) (* (`self.GetActorRightVector` _controlledcar_7) 2310.0))) (.y (+ (* (`self.GetActorForwardVector` _controlledcar_7) 6000.0) (* (`self.GetActorRightVector` _controlledcar_7) 2310.0))))) "BlockAll" false _array "ForOneFrame" true (struct :`R` 1.0 :`A` 1.0) (struct :`G` 1.0 :`A` 1.0) 0.05))
          (if _returnvalue_17
            (for _array_element_4 _outhits_4
              (bind (_bblockinghit_4 _binitialoverlap_4 _time_4 _distance_4 _location_4 _impactpoint_4 _normal_4 _impactnormal_4 _physmat_4 _hitactor_4) (`GameplayStatics.BreakHitResult` _array_element_4))
              (if (== "/Game/VehicleTemplate/Blueprints/Track.Track_C" (`GameplayStatics.GetObjectClass` _hitactor_4))
                (`self.Set Distance In Key` "topRight30" _distance_4)))))
        (:`then_4`
          ;[0 0 0] Top Left 30
          (bind (_outhits_5 _returnvalue_18) (`KismetSystemLibrary.LineTraceMultiByProfile` _returnvalue_13 (+ _returnvalue_13 (`KismetMathLibrary.MakeVector` (.x (+ (* (`self.GetActorForwardVector` _controlledcar_8) 6000.0) (* (`self.GetActorRightVector` _controlledcar_8) -2310.0))) (.y (+ (* (`self.GetActorForwardVector` _controlledcar_8) 6000.0) (* (`self.GetActorRightVector` _controlledcar_8) -2310.0))))) "BlockAll" false _array "ForOneFrame" true (struct :`R` 1.0 :`A` 1.0) (struct :`G` 1.0 :`A` 1.0) 0.05))
          (if _returnvalue_18
            (for _array_element_5 _outhits_5
              (bind (_bblockinghit_5 _binitialoverlap_5 _time_5 _distance_5 _location_5 _impactpoint_5 _normal_5 _impactnormal_5 _physmat_5 _hitactor_5) (`GameplayStatics.BreakHitResult` _array_element_5))
              (if (== "/Game/VehicleTemplate/Blueprints/Track.Track_C" (`GameplayStatics.GetObjectClass` _hitactor_5))
                (`self.Set Distance In Key` "topLeft30" _distance_5)))))
        (:`then_5`
          ;[0 0 0] Back
          (bind (_outhits_6 _returnvalue_19) (`KismetSystemLibrary.LineTraceMultiByProfile` _returnvalue_11 (+ _returnvalue_11 (`KismetMathLibrary.MakeVector` _returnvalue_x_2 _returnvalue_y_2)) "BlockAll" false _array "ForOneFrame" true (struct :`R` 1.0 :`A` 1.0) (struct :`G` 1.0 :`A` 1.0) 0.05))
          (if _returnvalue_19
            (for _array_element_6 _outhits_6
              (bind (_bblockinghit_6 _binitialoverlap_6 _time_6 _distance_6 _location_6 _impactpoint_6 _normal_6 _impactnormal_6 _physmat_6 _hitactor_6) (`GameplayStatics.BreakHitResult` _array_element_6))
              (if (== (`GameplayStatics.GetObjectClass` _hitactor_6) "/Game/VehicleTemplate/Blueprints/Track.Track_C")
                (`self.Set Distance In Key` "back" _distance_6)))))
        (:`then_6`
          ;[0 0 0] Bottom Right
          (bind (_outhits_7 _returnvalue_20) (`KismetSystemLibrary.LineTraceMultiByProfile` _returnvalue_8 (+ _returnvalue_8 (`KismetMathLibrary.MakeVector` (.x (+ (* (`self.GetActorForwardVector` _controlledcar_10) -4000.0) (* (`self.GetActorRightVector` _controlledcar_10) 4000.0))) (.y (+ (* (`self.GetActorForwardVector` _controlledcar_10) -4000.0) (* (`self.GetActorRightVector` _controlledcar_10) 4000.0))))) "BlockAll" false _array "ForOneFrame" true (struct :`R` 1.0 :`A` 1.0) (struct :`G` 1.0 :`A` 1.0) 0.05))
          (if _returnvalue_20
            (for _array_element_7 _outhits_7
              (bind (_bblockinghit_7 _binitialoverlap_7 _time_7 _distance_7 _location_7 _impactpoint_7 _normal_7 _impactnormal_7 _physmat_7 _hitactor_7) (`GameplayStatics.BreakHitResult` _array_element_7))
              (if (== (`GameplayStatics.GetObjectClass` _hitactor_7) "/Game/VehicleTemplate/Blueprints/Track.Track_C")
                (`self.Set Distance In Key` "bottomRight" _distance_7)))))
        (:`then_7`
          ;[0 0 0] Bottom Left
          (bind (_outhits_8 _returnvalue_21) (`KismetSystemLibrary.LineTraceMultiByProfile` _returnvalue_9 (+ _returnvalue_9 (`KismetMathLibrary.MakeVector` (.x (+ (* (`self.GetActorForwardVector` _controlledcar_11) -4000.0) (* (`self.GetActorRightVector` _controlledcar_11) -4000.0))) (.y (+ (* (`self.GetActorForwardVector` _controlledcar_11) -4000.0) (* (`self.GetActorRightVector` _controlledcar_11) -4000.0))))) "BlockAll" false _array "ForOneFrame" true (struct :`R` 1.0 :`A` 1.0) (struct :`G` 1.0 :`A` 1.0) 0.05))
          (if _returnvalue_21
            (for _array_element_8 _outhits_8
              (bind (_bblockinghit_8 _binitialoverlap_8 _time_8 _distance_8 _location_8 _impactpoint_8 _normal_8 _impactnormal_8 _physmat_8 _hitactor_8) (`GameplayStatics.BreakHitResult` _array_element_8))
              (if (== "/Game/VehicleTemplate/Blueprints/Track.Track_C" (`GameplayStatics.GetObjectClass` _hitactor_8))
                (`self.Set Distance In Key` "bottomLeft" _distance_8)))))
        (:`then_8`
          ;[0 0 0] Bottom Right 30
          (bind (_outhits_9 _returnvalue_22) (`KismetSystemLibrary.LineTraceMultiByProfile` _returnvalue_10 (+ _returnvalue_10 (`KismetMathLibrary.MakeVector` (.x (+ (* (`self.GetActorForwardVector` _controlledcar_13) -6000.0) (* (`self.GetActorRightVector` _controlledcar_13) 2310.0))) (.y (+ (* (`self.GetActorForwardVector` _controlledcar_13) -6000.0) (* (`self.GetActorRightVector` _controlledcar_13) 2310.0))))) "BlockAll" false _array "ForOneFrame" true (struct :`R` 1.0 :`A` 1.0) (struct :`G` 1.0 :`A` 1.0) 0.05))
          (if _returnvalue_22
            (for _array_element_9 _outhits_9
              (bind (_bblockinghit_9 _binitialoverlap_9 _time_9 _distance_9 _location_9 _impactpoint_9 _normal_9 _impactnormal_9 _physmat_9 _hitactor_9) (`GameplayStatics.BreakHitResult` _array_element_9))
              (if (== "/Game/VehicleTemplate/Blueprints/Track.Track_C" (`GameplayStatics.GetObjectClass` _hitactor_9))
                (`self.Set Distance In Key` "bottomRight30" _distance_9)))))
        (:`then_9`
          ;[0 0 0] Bottom Left 30
          (bind (_outhits_10 _returnvalue_23) (`KismetSystemLibrary.LineTraceMultiByProfile` _returnvalue (+ _returnvalue (`KismetMathLibrary.MakeVector` (.x (+ (* (`self.GetActorForwardVector` _controlledcar_12) -6000.0) (* (`self.GetActorRightVector` _controlledcar_12) -2310.0))) (.y (+ (* (`self.GetActorForwardVector` _controlledcar_12) -6000.0) (* (`self.GetActorRightVector` _controlledcar_12) -2310.0))))) "BlockAll" false _array "ForOneFrame" true (struct :`R` 1.0 :`A` 1.0) (struct :`G` 1.0 :`A` 1.0) 0.05))
          (if _returnvalue_23
            (for _array_element_10 _outhits_10
              (bind (_bblockinghit_10 _binitialoverlap_10 _time_10 _distance_10 _location_10 _impactpoint_10 _normal_10 _impactnormal_10 _physmat_10 _hitactor_10) (`GameplayStatics.BreakHitResult` _array_element_10))
              (if (== "/Game/VehicleTemplate/Blueprints/Track.Track_C" (`GameplayStatics.GetObjectClass` _hitactor_10))
                (`self.Set Distance In Key` "bottomLeft30" _distance_10)))))
        (:`then_10`
          ;[0 0 0] Left
          (bind (_outhits_11 _returnvalue_24) (`KismetSystemLibrary.LineTraceMultiByProfile` :`Start` _returnvalue_2 :`End` (+ _returnvalue_2 (`KismetMathLibrary.MakeVector` (.x (* (`self.GetActorRightVector` _controlledcar_4) -2500.0)) (.y (* (`self.GetActorRightVector` _controlledcar_4) -2500.0)))) :`ProfileName` "BlockAll" :`DrawDebugType` "ForOneFrame" :`DrawTime` 0.05))
          (if _returnvalue_24
            (for _array_element_11 _outhits_11
              (bind (_bblockinghit_11 _binitialoverlap_11 _time_11 _distance_11 _location_11 _impactpoint_11 _normal_11 _impactnormal_11 _physmat_11 _hitactor_11) (`GameplayStatics.BreakHitResult` _array_element_11))
              (if (== "/Game/VehicleTemplate/Blueprints/Track.Track_C" (`GameplayStatics.GetObjectClass` _hitactor_11))
                (`self.Set Distance In Key` "left" _distance_11)))))
        (:`then_11`
          ;[0 0 0] Right
          (bind (_outhits_12 _returnvalue_25) (`KismetSystemLibrary.LineTraceMultiByProfile` :`Start` _returnvalue_3 :`End` (+ _returnvalue_3 (`KismetMathLibrary.MakeVector` (.x (* (`self.GetActorRightVector` _controlledcar_5) 2500.0)) (.y (* (`self.GetActorRightVector` _controlledcar_5) 2500.0)))) :`ProfileName` "BlockAll" :`DrawDebugType` "ForOneFrame" :`DrawTime` 0.05))
          (if _returnvalue_25
            (for _array_element_12 _outhits_12
              (bind (_bblockinghit_12 _binitialoverlap_12 _time_12 _distance_12 _location_12 _impactpoint_12 _normal_12 _impactnormal_12 _physmat_12 _hitactor_12) (`GameplayStatics.BreakHitResult` _array_element_12))
              (if (== "/Game/VehicleTemplate/Blueprints/Track.Track_C" (`GameplayStatics.GetObjectClass` _hitactor_12))
                (`self.Set Distance In Key` "right" _distance_12)))))
        (:`then_12`
          ;[0 0 0] Down
          (bind (_outhits_13 _returnvalue_26) (`KismetSystemLibrary.LineTraceMultiByProfile` :`Start` _returnvalue_6 :`End` (+ _returnvalue_6 (`KismetMathLibrary.MakeVector` (.x (* (`self.GetActorUpVector` _controlledcar_9) -1000.0)) (.y (* (`self.GetActorUpVector` _controlledcar_9) -1000.0)) (.z (* (`self.GetActorUpVector` _controlledcar_9) -1000.0)))) :`ProfileName` "BlockAll" :`DrawDebugType` "ForOneFrame" :`DrawTime` 0.05))
          (if _returnvalue_26
            (for _array_element_13 _outhits_13
              (bind (_bblockinghit_13 _binitialoverlap_13 _time_13 _distance_13 _location_13 _impactpoint_13 _normal_13 _impactnormal_13 _physmat_13 _hitactor_13) (`GameplayStatics.BreakHitResult` _array_element_13))
              (if (== "/Game/VehicleTemplate/Blueprints/Track.Track_C" (`GameplayStatics.GetObjectClass` _hitactor_13))
                (`self.Set Distance In Key` "bottom" _distance_13)))))
        (:`then_13`
          (goto _label))))))

(fn `Accelerate`
  (params (`Action Value` :type "Float (double-precision)"))
  (bind _asaisports_car_pawn (cast `/Game/AI/AISportsCar_Pawn` (`self.K2_GetPawn`)))
  (`/Game/AI/AISportsCar_Pawn.Throttle` _asaisports_car_pawn `Action Value`)
  (return))

(fn `Break`
  (params (`Action Value` :type "Float (double-precision)"))
  (bind _asaisports_car_pawn (cast `/Game/AI/AISportsCar_Pawn` (`self.K2_GetPawn`)))
  (`/Game/AI/AISportsCar_Pawn.Break` _asaisports_car_pawn `Action Value`)
  (return))

(fn `Set Distance In Key`
  (params (`In Key` :type "ELinecastDirections Enum" :default "front") (`New Distance ` :type "Float (single-precision)"))
  (`|VariableSetRef` (`|GetArrayItem` (`self.Distances`) (`KismetArrayLibrary.Array_Find` (`self.Directions`) `In Key`)) `New Distance `)
  (return))

(fn `Steer`
  (params (`Action Value` :type "Float (double-precision)"))
  (bind _asaisports_car_pawn (cast `/Game/AI/AISportsCar_Pawn` (`self.K2_GetPawn`)))
  (`/Game/AI/AISportsCar_Pawn.Steering` _asaisports_car_pawn `Action Value`)
  (return))

(fn `UserConstructionScript`
  (`parent.UserConstructionScript`))