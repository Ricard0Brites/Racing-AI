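; Neural network Blueprint for the NotFastJustFurious AI team, currently set up as a test harness for the parent class's network functions.
; On BeginPlay it initializes a three-hidden-layer network, attempts to load saved values, then feeds a hard-coded test input after a short delay.
; NeuralOutput prints each result, and ActivationFunction supplies a sigmoid.
; Incentivise, Punish, save and reset calls are present but never run.
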(event `self.ReceiveBeginPlay`
  (`parent.ReceiveBeginPlay`)
  (`KismetSystemLibrary.Delay` 0.0)
  (`self.InitNeuralNetwork` 13 3 9 3)
  (`|ExecutionSequence`
    (:`then_0`
      (bind _returnvalue (`self.LoadNeuralNetworkValues`))
      (if _returnvalue
        (`KismetSystemLibrary.PrintString` "NN Was Loaded Successfully " true true (struct :`G` 1.0 :`A` 1.0))
        (else
          (`KismetSystemLibrary.PrintString` "NN Was't Loaded" true true (struct :`R` 1.0 :`A` 1.0)))))
    (:`then_1`
      (`KismetSystemLibrary.Delay` 1.0)
      (`self.NeuralInput` (`|MakeArray` 20.0 50.0 100.0 200.0 500.0 1.0 5.0 2.0 5.0 4.0 2.0 0.0 3.0 :!type "Float (single-precision)")))))

(event `self.NeuralOutput`
  (params (Out :type "Array of Float (single-precision) (by ref)"))
  (for _array_element Out
    (`KismetSystemLibrary.PrintString` (`KismetStringLibrary.Conv_DoubleToString` _array_element) true true (struct :`G` 0.66 :`B` 1.0 :`A` 1.0) 50.0)))

(fn `ActivationFunction`
  (params (Input :type "Float (single-precision)"))
  (returns (ReturnValue :type "Float (single-precision)"))
  (return (/ 1.0 (+ 1.0 (`KismetMathLibrary.Exp` (* Input -1.0))))))

(fn `UserConstructionScript`
  (`parent.UserConstructionScript`))