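; AI car controller for the NotFastJustFurious team that maps the track into waypoints at BeginPlay.
; It spawns a temporary barrier behind the car, then walks along the track wall with line traces, periodically spawning linked BP_Waypoints until it hits a TrackEnd-tagged actor.
; Helpers forward throttle, brake and steering to the AISportsCar pawn.
; Alg1, a raycast-distance steering loop, is never run, and RaceStarted is empty, so nothing here drives the car.
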(event `self.ReceivePossess`
  (params (PossessedPawn :type "Pawn Object Reference"))
  (`parent.ReceivePossess` PossessedPawn))

(event `Delete Barrier`
  (`self.K2_DestroyActor` (stale `self.ReceiveBeginPlay` _returnvalue_2)))

(event `self.ReceiveBeginPlay`
  (bind _trace_length (`self.Trace Length`))
  (bind _trace_offset (`self.Trace Offset`))
  (bind _trace_interval (`self.Trace Interval`))
  (bind _controlledcar (`self.ControlledCar`))
  (bind _controlledcar_2 (`self.ControlledCar`))
  (bind (_returnvalue_x _returnvalue_y) (`KismetMathLibrary.BreakVector` (`self.K2_GetActorLocation` _controlledcar)))
  (bind _returnvalue (`KismetMathLibrary.MakeVector` _returnvalue_x _returnvalue_y 12.0))
  (bind (_returnvalue_x_2 _returnvalue_y_2) (`KismetMathLibrary.BreakVector` (* (`self.GetActorRightVector` _controlledcar) (select `bool` (< (`KismetMathLibrary.FMax` (.x (`self.GetActorRightVector` (`self.ControlledCar`))) (.y (`self.GetActorRightVector` (`self.ControlledCar`)))) 0.0) :`false` 4000.0 :`true` -4000.0 :!type "Float (single-precision)"))))
  (`|ExecutionSequence`
    (:`then_0`
      (bind _returnvalue_2 (`|SpawnActorFromClass` "/Game/AI/AITeams/NotFastJustFurious/BP_Barrier.BP_Barrier_C" (`KismetMathLibrary.MakeTransform` (+ (* (`self.GetActorForwardVector` _controlledcar_2) -100) (`self.K2_GetActorLocation` _controlledcar_2)) (`self.K2_GetActorRotation` _controlledcar_2)) "AlwaysSpawn" "OverrideRootScale" null null)))
    (:`then_1`
      (bind (_outhit _returnvalue_3) (`KismetSystemLibrary.LineTraceSingleByProfile` _returnvalue (+ _returnvalue (`KismetMathLibrary.MakeVector` _returnvalue_x_2 _returnvalue_y_2)) "BlockAll" false (`|MakeArray` _controlledcar :!type "Actor Object Reference") (`self.Draw Debug Type`)))
      (if _returnvalue_3
        (bind (_bblockinghit _binitialoverlap _time _distance _location _impactpoint _normal) (`GameplayStatics.BreakHitResult` _outhit))
        (bind _returnvalue_4 (+ (* (`self.GetActorForwardVector` (`self.ControlledCar`)) (`KismetMathLibrary.MakeVector` _trace_interval _trace_interval)) (- _impactpoint (* (`self.GetActorRightVector` (`self.ControlledCar`)) (`KismetMathLibrary.MakeVector` _trace_offset _trace_offset)))))
        (bind _outhit_2 (`KismetSystemLibrary.LineTraceSingleByProfile` :`Start` _returnvalue_4 :`End` (+ _returnvalue_4 (* _normal (`KismetMathLibrary.MakeVector` _trace_length _trace_length))) :`ProfileName` "BlockAll" :`DrawDebugType` (`self.Draw Debug Type`)))
        (set `self.Last Hit` _outhit_2)
        (`self.Trace Track`)))))

(event `Trace Track`
  (bind _trace_offset (`self.Trace Offset`))
  (bind _last_waypoint (`self.Last Waypoint`))
  (bind _trace_length (`self.Trace Length`))
  (bind _trace_offset_2 (`self.Trace Offset`))
  (bind (_last_hit_bblockinghit _last_hit_binitialoverlap _last_hit_time _last_hit_distance _last_hit_location _last_hit_impactpoint _last_hit_normal _last_hit_impactnormal _last_hit_physmat _last_hit_hitactor _last_hit_hitcomponent _last_hit_hitbonename _last_hit_bonename _last_hit_hititem _last_hit_elementindex _last_hit_faceindex _last_hit_tracestart _last_hit_traceend) (`GameplayStatics.BreakHitResult` (`self.Last Hit`)))
  (bind _trace_interval (`self.Trace Interval`))
  (bind (_bblockinghit _binitialoverlap _time _distance _location _impactpoint _normal) (`GameplayStatics.BreakHitResult` (`self.Last Hit`)))
  (bind (_bblockinghit_2 _binitialoverlap_2 _time_2 _distance_2 _location_2 _impactpoint_2 _normal_2) (`GameplayStatics.BreakHitResult` (`self.Last Hit`)))
  (bind (_bblockinghit_3 _binitialoverlap_3 _time_3 _distance_3 _location_3 _impactpoint_3 _normal_3) (`GameplayStatics.BreakHitResult` (`self.Last Hit`)))
  (bind _returnvalue (+ _impactpoint (* _normal (`KismetMathLibrary.MakeVector` _trace_offset _trace_offset))))
  (bind _returnvalue_2 (+ _impactpoint_3 (* _normal_3 (10.0 10.0 0.0))))
  (bind _returnvalue_3 (+ (+ _impactpoint_2 (* _normal_2 (`KismetMathLibrary.MakeVector` _trace_offset_2 _trace_offset_2))) (* (`self.Rotate Vector 90` _normal_2) (500.0 500.0 0.0))))
  (while (not (`self.Has Finished Tracing`))
    (`/Engine/EditorBlueprintResources/StandardMacros.IncrementInt` (`self.Loop Counter`)
      (:`  `
        (bind (_outhit _returnvalue_4) (`KismetSystemLibrary.LineTraceSingle` :`Start` _returnvalue :`End` (+ _returnvalue (* (`self.Rotate Vector 90` _normal) (`KismetMathLibrary.MakeVector` _trace_interval _trace_interval))) :`TraceChannel` "TraceTypeQuery1" :`DrawDebugType` (`self.Draw Debug Type`)))
        (if _returnvalue_4
          (if (not (`self.ActorHasTag` (`.HitActor` (`GameplayStatics.BreakHitResult` _outhit)) "TrackEnd"))
            (bind (_outhit_2 _returnvalue_5) (`KismetSystemLibrary.LineTraceSingleByProfile` :`Start` _returnvalue_3 :`End` (+ _returnvalue_3 (* _normal_2 (`KismetMathLibrary.MakeVector` _trace_length _trace_length))) :`ProfileName` "BlockAll" :`DrawDebugType` (`self.Draw Debug Type`) :!label _label))
            (if _returnvalue_5
              (set `self.Last Hit` _outhit_2)
              (if (>= (`self.Loop Counter`) (`self.Place Gate Each X Traces`))
                (set `self.Loop Counter` 0)
                (bind _outhit_3 (`KismetSystemLibrary.LineTraceSingleByProfile` :`Start` _returnvalue_2 :`End` (+ _returnvalue_2 (* _normal_3 (4000.0 4000.0 0.0))) :`ProfileName` "BlockAll" :`DrawDebugType` (`self.Draw Debug Type`)))
                (bind (_bblockinghit_4 _binitialoverlap_4 _time_4 _distance_4 _location_4 _impactpoint_4 _normal_4 _impactnormal _physmat _hitactor _hitcomponent _hitbonename _bonename _hititem _elementindex _faceindex _tracestart _traceend) (`GameplayStatics.BreakHitResult` _outhit_3))
                (bind _returnvalue_6 (`|SpawnActorFromClass` "/Game/AI/AITeams/NotFastJustFurious/BP_Waypoint.BP_Waypoint_C" (`KismetMathLibrary.MakeTransform` (+ _returnvalue_2 (* _normal_3 (`KismetMathLibrary.MakeVector` _distance_4 _distance_4))) (`KismetMathLibrary.MakeRotFromX` (`self.Rotate Vector 90` (- _traceend _tracestart)))) "AlwaysSpawn" "OverrideRootScale" null null))
                (`/Engine/EditorBlueprintResources/StandardMacros.IsValid` _last_waypoint
                  (:`Is Valid`
                    (set `/Game/AI/AITeams/NotFastJustFurious/BP_Waypoint.Next Waypoint` _returnvalue_6 _last_waypoint))
                  (:`Is Not Valid`
                    (set `self.First Waypoint` _returnvalue_6)))
                (set `self.Last Waypoint` _returnvalue_6))
              (else
                (set `self.Last Hit` (`GameplayStatics.MakeHitResult` _last_hit_bblockinghit _last_hit_binitialoverlap _last_hit_time _last_hit_distance _last_hit_location (+ _last_hit_impactpoint (* _last_hit_normal (-10.0 -10.0 0.0))) _last_hit_normal _last_hit_impactnormal _last_hit_physmat _last_hit_hitactor _last_hit_hitcomponent _last_hit_hitbonename _last_hit_bonename _last_hit_hititem _last_hit_elementindex _last_hit_faceindex _last_hit_tracestart _last_hit_traceend))))
            (else
              (set `self.Has Finished Tracing` true)
              (`self.Delete Barrier`)
              (set `/Game/AI/AITeams/NotFastJustFurious/BP_Waypoint.Next Waypoint` (`self.Last Waypoint`) (`self.First Waypoint`))))
          (else
            (goto _label))))))
  (set `self.Next Waypoint` (`self.First Waypoint`)))

(event `self.Race Started`)

(fn `Accelerate`
  (params (`Action Value` :type "Float (double-precision)"))
  (bind _asaisports_car_pawn (cast `/Game/AI/AISportsCar_Pawn` (`self.K2_GetPawn`)))
  (`/Game/AI/AISportsCar_Pawn.Throttle` _asaisports_car_pawn `Action Value`)
  (return))

(fn `Break`
  (params (`Action Value` :type "Float (double-precision)"))
  (bind _asaisports_car_pawn (cast `/Game/AI/AISportsCar_Pawn` (`self.K2_GetPawn`)))
  (`/Game/AI/AISportsCar_Pawn.Break` _asaisports_car_pawn `Action Value`)
  (return))

(fn `Get Angle Between Vectors`
  (params (U :type "Vector Structure") (V :type "Vector Structure"))
  (returns (Angle :type "Float (double-precision)"))
  (bind _x (.x U))
  (bind _y (.y U))
  (bind _x_2 (.x V))
  (bind _y_2 (.y V))
  (return (+ (`KismetMathLibrary.DegAtan2` (- (* _x _y_2) (* _y _x_2)) (+ (* _x _x_2) (* _y _y_2))) 180.0)))

(fn `Get Distance`
  (params (ItemToFind :type "ELinecastDirections Enum" :default "front"))
  (returns (Output :type "Float (double-precision) (by ref)"))
  (return (`|GetArrayItem` (`self.Distances`) (`KismetArrayLibrary.Array_Find` (`self.Directions`) ItemToFind))))

(fn `Is Between?`
  (params (Number :type "Float (double-precision)") (A :type "Float (double-precision)") (B :type "Float (double-precision)"))
  (returns (ReturnValue :type Boolean))
  (return (and (<= A Number) (>= B Number))))

(fn `Rotate Vector 90`
  (params (`In Vec` :type "Vector Structure"))
  (returns (ReturnValue :type "Vector Structure"))
  (return (* (`KismetMathLibrary.MakeVector` `In Vec_Y` (* `In Vec_X` -1.0) `In Vec_Z`) -1)))

(fn `Set Distance In Key`
  (params (`In Key` :type "ELinecastDirections Enum" :default "front") (`New Distance ` :type "Float (single-precision)"))
  (`|VariableSetRef` (`|GetArrayItem` (`self.Distances`) (`KismetArrayLibrary.Array_Find` (`self.Directions`) `In Key`)) `New Distance `)
  (return))

(fn `Steer`
  (params (`Action Value` :type "Float (double-precision)"))
  (bind _asaisports_car_pawn (cast `/Game/AI/AISportsCar_Pawn` (`self.K2_GetPawn`)))
  (`/Game/AI/AISportsCar_Pawn.Steering` _asaisports_car_pawn `Action Value`)
  (return))

(fn `UserConstructionScript`
  (`parent.UserConstructionScript`))