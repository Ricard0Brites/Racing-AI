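; Racing AI waypoint gate that feeds throttle and brake values to the team's car controller.
; When the car overlaps the active gate, it activates the next, cuts acceleration at full steering lock and applies its values.
; Reward and punish events nudge those values as simple learning, but save/load logic is disconnected.
; At start, side traces from two gates ahead shift the actor toward the nearer hit, leaving its trigger box in place.
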(event `self.ReceiveBeginPlay`
  (bind _next_waypoint (`self.Get Next Waypoint` (`self.Get Next Waypoint`)))
  (bind _returnvalue (`self.K2_GetActorLocation` _next_waypoint))
  (bind _returnvalue_2 (`self.GetActorRightVector` _next_waypoint))
  (`KismetSystemLibrary.Delay` 0.0) ; wait 1 frame so all of the waypoints\nAre created
  (set `self.Acceleration` 1.0)
  (set `self.Braking` 0.0)
  (`self.Load Values`)
  (bind _outhit (`KismetSystemLibrary.LineTraceSingleByProfile` _returnvalue (+ _returnvalue (* _returnvalue_2 2000)) "BlockAll"))
  (bind (_bblockinghit _binitialoverlap _time _distance _location _impactpoint _normal _impactnormal _physmat _hitactor _hitcomponent _hitbonename _bonename _hititem _elementindex _faceindex _tracestart) (`GameplayStatics.BreakHitResult` _outhit))
  (bind _outhit_2 (`KismetSystemLibrary.LineTraceSingleByProfile` _tracestart (+ _tracestart (* _returnvalue_2 -2000)) "BlockAll"))
  (bind _returnvalue_3 (- (`.ImpactPoint` (`GameplayStatics.BreakHitResult` _outhit_2)) (`self.K2_GetActorLocation`)))
  (bind _returnvalue_4 (- (`.ImpactPoint` (`GameplayStatics.BreakHitResult` _outhit)) (`self.K2_GetActorLocation`)))
  (`self.Offset Actor` (- (select `bool` (> (`KismetMathLibrary.VSize` _returnvalue_3) (`KismetMathLibrary.VSize` _returnvalue_4)) :`false` _returnvalue_3 :`true` _returnvalue_4) (* _returnvalue_2 -350))))

(event `self.Box.OnComponentBeginOverlap`
  (params (OverlappedComponent :type "PrimitiveComponent Object Reference") (OtherActor :type "Actor Object Reference") (OtherComp :type "PrimitiveComponent Object Reference") (OtherBodyIndex :type Integer) (bFromSweep :type Boolean) (SweepResult :type "HitResult Structure (by ref)"))
  ;[0 0 0] If other object is My Car
  (if (and (== OtherActor (`self.My Car Reference`)) (`self.Is Waypoint Active?`))
    (`|ExecutionSequence`
      (:`then_0`
        ;[0 0 0] Activate next Gate
        (`self.Activate Next Waypoint`)
        (set `/Game/AI/AITeams/NotFastJustFurious/BP_CarController.Next Waypoint` (`self.Next Waypoint`) (`self.Controller Reference`)))
      (:`then_1`
        (bind _returnvalue (`ChaosVehicleMovementComponent.GetSteeringInput` (`WheeledVehiclePawn.VehicleMovementComponent` (`self.My Car Reference`))))
        (if (== 1.0 (`KismetMathLibrary.Abs` _returnvalue))
          (set `self.Acceleration` 0.1)))
      (:`then_2`
        ;[0 0 0] Reward AI
        (if (`/Game/AI/AITeams/NotFastJustFurious/BP_CarController.Is Learning Enabled` (`self.Controller Reference`))
          (`self.Reward AI`)))
      (:`then_3`
        ;[0 0 0] Feed the AI the new Values
        (`self.Set Acceleration` (`self.Acceleration`))
        (`self.Set Braking` (`self.Braking`))))))

(event `Punish AI`
  (`|ExecutionSequence`
    (:`then_0`
      (`self.Offset Acceleration` (* 0.01 -1.0)))
    (:`then_1`
      (`self.Offset Braking` 0.01)))
  (`self.Save Values` :!label _label))

(event `Reward AI`
  (if (`KismetMathLibrary.RandomBool`)
    (`self.Offset Acceleration` 0.001)
    (goto _label)
    (else
      (`self.Offset Braking` (* 0.001 -1.0))
      (goto _label))))

(event `Load Values`)

(event `Save Values`)

(event `Delete Save`
  (`GameplayStatics.DeleteGameInSlot` "NotFastJustFurious"))

(fn `Activate Next Waypoint`
  (set `/Game/AI/AITeams/NotFastJustFurious/BP_Waypoint.Is Waypoint Active?` true (`self.Next Waypoint`))
  (set `self.Is Waypoint Active?` false)
  (return))

(fn `Get Car Controls`
  (returns (Braking :type "Float (single-precision)") (Acceleration :type "Float (single-precision)"))
  (bind _vehiclemovementcomponent (`WheeledVehiclePawn.VehicleMovementComponent` (`self.My Car Reference`)))
  (bind _returnvalue (`ChaosVehicleMovementComponent.GetBrakeInput` _vehiclemovementcomponent))
  (bind _returnvalue_2 (`ChaosVehicleMovementComponent.GetThrottleInput` _vehiclemovementcomponent))
  (return _returnvalue _returnvalue_2))

(fn `Get Next Waypoint`
  (returns (`Next Waypoint` :type "/Game/AI/AITeams/NotFastJustFurious/BP_Waypoint Object Reference"))
  (return (`self.Next Waypoint`)))

(fn `Offset Acceleration`
  (params (Offset :type "Float (double-precision)"))
  (returns (`New Value` :type "Float (double-precision)"))
  (bind _returnvalue (`KismetMathLibrary.FClamp` (+ (`self.Acceleration`) Offset)))
  (`/Game/AI/AITeams/NotFastJustFurious/BP_CarController.Accelerate` (`self.Controller Reference`) _returnvalue)
  (set `self.Acceleration` _returnvalue)
  (return _returnvalue))

(fn `Offset Actor`
  (params (Offset :type "Vector Structure"))
  (bind _box (`self.Box`))
  (bind _output_get (set `self.Collider Location` (`SceneComponent.K2_GetComponentLocation` _box)))
  (`self.K2_AddActorWorldOffset` Offset false true)
  (`SceneComponent.K2_SetWorldLocation` _box _output_get false true)
  (set `self.Actor Ofset` (+ Offset (`self.Actor Ofset`))))

(fn `Offset Braking`
  (params (Offset :type "Float (double-precision)"))
  (returns (`New Value` :type "Float (double-precision)"))
  (bind _returnvalue (`KismetMathLibrary.FClamp` (+ (`self.Braking`) Offset)))
  (`/Game/AI/AITeams/NotFastJustFurious/BP_CarController.Brake` (`self.Controller Reference`) _returnvalue)
  (set `self.Braking` _returnvalue)
  (return _returnvalue))

(fn `Set Acceleration`
  (params (`Action Value` :type "Float (double-precision)"))
  (`/Game/AI/AITeams/NotFastJustFurious/BP_CarController.Accelerate` (`self.Controller Reference`) `Action Value`)
  (set `self.Acceleration` `Action Value`)
  (return))

(fn `Set Braking`
  (params (`Action Value` :type "Float (double-precision)"))
  (`/Game/AI/AITeams/NotFastJustFurious/BP_CarController.Brake` (`self.Controller Reference`) `Action Value`)
  (set `self.Braking` `Action Value`)
  (return))

(fn `UserConstructionScript`)